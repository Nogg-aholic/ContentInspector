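; Chat command that opens the mod's inspector windows for content or for a targeted actor.
; With the "this" argument, it line-traces from the player's view, opens an Actor Inspector on the hit actor and reports the hit or miss in chat.
; Otherwise it restores the minimized inspector held by the ContentInspector_InitWorld world module, or creates a new Content Inspector if none is valid.
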(fn `ExecuteCommand`
  (params (Sender :type "CommandSender Object Reference") (Arguments :type "Array of String (by ref)") (Label :type String))
  (returns (ReturnValue :type "EExecutionStatus Enum"))
  (locals (Recipes :type "Array of FGRecipe Class Reference") (Items :type "Array of FGItemDescriptor Class Reference") (class :type "Array of Object Class Reference") (NewLocalVar_0 :type "Object Class Reference" :default "Class'/Script/CoreUObject.Class'") (Class_0 :type "Array of Object Class Reference"))
  (bind _returnvalue (`Controller.K2_GetPawn` (`CommandSender.GetPlayer` Sender)))
  (bind (_outlocation _outrotation) (`self.GetActorEyesViewPoint` _returnvalue))
  (bind _minimized_window (`/ContentInspector/ContentInspector_InitWorld.Minimized Window` (cast `/ContentInspector/ContentInspector_InitWorld` (`WorldModuleManager.FindModule` (subsystem `WorldModuleManager`) (`self.GetOwnerModReference`)) :!pure true)))
  (if (`KismetStringLibrary.EqualEqual_StrStr` (`|GetArrayItem` Arguments) "this")
    (bind (_outhit _returnvalue_2) (`KismetSystemLibrary.LineTraceSingleForObjects` _outlocation (+ _outlocation (* (`KismetMathLibrary.GetForwardVector` _outrotation) (`self.Distance`))) (`|MakeArray` "ObjectTypeQuery1" "ObjectTypeQuery2" "ObjectTypeQuery6" "ObjectTypeQuery9" "ObjectTypeQuery3" "ObjectTypeQuery4" "ObjectTypeQuery5" "ObjectTypeQuery7" "ObjectTypeQuery8" "ObjectTypeQuery14" :!type "EObjectTypeQuery Enum") false (`|MakeArray` _returnvalue :!type "Actor Object Reference") "ForDuration" true (struct :`R` 1.0 :`A` 1.0) (struct :`G` 1.0 :`A` 1.0) 1.0))
    (if _returnvalue_2
      (bind (_bblockinghit _binitialoverlap _time _distance _location _impactpoint _normal _impactnormal _physmat _hitactor _hitcomponent) (`GameplayStatics.BreakHitResult` _outhit))
      (bind _returnvalue_3 (`|CreateWidget` "/ContentInspector/Widgets/Widget_ActorInspector.Widget_ActorInspector_C" null _hitactor))
      (`UserWidget.AddToViewport` _returnvalue_3 0)
      (bind _result (`|FormatText` "Opened actor {ActorName} (hit at distance {Distance} on component {Component})" (`KismetSystemLibrary.GetDisplayName` _hitactor) _distance (`KismetSystemLibrary.GetDisplayName` _hitcomponent)))
      (`/ContentInspector/Widgets/Widget_ActorInspector.Display Message` _returnvalue_3 _result 0.0)
      (`CommandSender.SendChatMessage` Sender (`KismetTextLibrary.Conv_TextToString` _result) (struct :`G` 1.0 :`A` 1.0))
      (return "COMPLETED")
      (else
        (`CommandSender.SendChatMessage` Sender "Trace for actors didn't hit anything" (struct :`G` 1.0 :`A` 1.0))
        (return "UNCOMPLETED")))
    (else
      (`/Engine/EditorBlueprintResources/StandardMacros.IsValid` _minimized_window
        (:`Is Valid`
          (bind _aswidget_content_inspector (cast `/ContentInspector/Widgets/Widget_ContentInspector` _minimized_window)
            (:`then`
              (`/ContentInspector/Widgets/Widget_ContentInspector.Restore from Minimize` _aswidget_content_inspector "Restored from minimized"))
            (:`CastFailed`
              (bind _aswidget_actor_inspector (cast `/ContentInspector/Widgets/Widget_ActorInspector` _minimized_window)
                (:`then`
                  (`/ContentInspector/Widgets/Widget_ActorInspector.Restore from Minimize` _aswidget_actor_inspector "Restored from minimized"))
                (:`CastFailed`
                  (return "UNCOMPLETED"))))))
        (:`Is Not Valid`
          (bind _returnvalue_4 (`|CreateWidget` "/ContentInspector/Widgets/Widget_ContentInspector.Widget_ContentInspector_C"))
          (`UserWidget.AddToViewport` _returnvalue_4 0)))
      (return "COMPLETED"))))

(fn `UserConstructionScript`)